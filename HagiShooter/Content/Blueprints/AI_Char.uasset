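; AI character that carries a gun, shoots a given enemy and can be killed.
; On BeginPlay it snaps the gun mesh to the character's weapon socket.
; ShootEnemy spawns an emitter at the gun socket, line traces for Pawns toward the target and sends a fixed-damage TakeDamage message to the actor hit.
; Its own TakeDamage event lowers Health and destroys the actor at zero or below.
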(event `self.ReceiveBeginPlay`
  ;[1 1 1] Set Start Gun Animation
  (`SceneComponent.K2_AttachToComponent` (`self.GunMesh`) (`self.Mesh`) "WeaponSocket" "SnapToTarget" "SnapToTarget" "SnapToTarget" true))

(event `Shoot Enemy`
  (params (EnemyToShoot :type "Actor Object Reference"))
  ;[1 1 1] Shoot At Player
  (`self.Play Shoot FX`)
  (bind _outhit (`KismetSystemLibrary.LineTraceSingleForObjects` (`self.K2_GetActorLocation`) (`self.K2_GetActorLocation` EnemyToShoot) (`|MakeArray` "ObjectTypeQuery3" :!type "EObjectTypeQuery Enum")))
  (bind (_bblockinghit _binitialoverlap _time _distance _location _impactpoint _normal _impactnormal _physmat _hitactor) (`GameplayStatics.BreakHitResult` _outhit))
  (if _bblockinghit
    (message `/Game/Blueprints/TakeDamage.Take Damage` _hitactor 5)))

(event `Play Shoot FX`
  (bind _gunmesh (`self.GunMesh`))
  ;[1 1 1] Shoot FX
  (`GameplayStatics.SpawnEmitterAtLocation` null (`SceneComponent.GetSocketLocation` _gunmesh "Socket") (`SceneComponent.GetSocketRotation` _gunmesh "Socket")))

(event `/Game/Blueprints/TakeDamage.Take Damage`
  (params (Damage :type Integer))
  ;[1 1 1] AI Take Damage
  (bind _output_get (set `self.Health` (- (`self.Health`) (`KismetMathLibrary.Conv_IntToDouble` Damage))))
  (if (<= _output_get 0.0)
    (`self.K2_DestroyActor`)))

(fn `UserConstructionScript`)