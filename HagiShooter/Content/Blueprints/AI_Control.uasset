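; AI controller that runs the AI_Character behavior tree on possession and tracks the player as its enemy.
; BeginPlay caches player character 0 and writes it to the blackboard as Enemy.
; AI Perception updates set CanSeePlayer from the player's first last-sensed stimulus.
; When sensing fails, it stores the player's current location as LastSeenLocation and draws a debug sphere there.
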(event `self.ReceiveBeginPlay`
  (bind _returnvalue (`GameplayStatics.GetPlayerCharacter` 0))
  (set `self.Enemy` _returnvalue)
  (`BlackboardComponent.SetValueAsObject` (`AIBlueprintHelperLibrary.GetBlackboard` null) "Enemy" _returnvalue))

(event `self.ReceivePossess`
  (params (PossessedPawn :type "Pawn Object Reference"))
  (`self.UseBlackboard` "/Game/Blueprints/BB_AICharacter.BB_AICharacter")
  (`self.RunBehaviorTree` "/Game/Blueprints/AI_Character.AI_Character"))

(event `self.AIPerception.OnPerceptionUpdated`
  (params (UpdatedActors :type "Array of Actor Object Reference (by ref)"))
  (bind _returnvalue (`AIBlueprintHelperLibrary.GetBlackboard` null))
  (bind _returnvalue_2 (`self.K2_GetActorLocation` (`self.Enemy`)))
  ;[1 1 1] Last Seen Location
  (for _array_element UpdatedActors
    (if (== _array_element (`self.Enemy`))
      (bind _info (`AIPerceptionComponent.GetActorsPerception` (`self.AIPerception`) _array_element))
      (bind (_age _expirationage _strength _stimuluslocation _receiverlocation _tag _bsuccessfullysensed) (break `AIStimulus` (`|GetArrayItem` (`.LastSensedStimuli` (break `ActorPerceptionBlueprintInfo` _info)))))
      (`BlackboardComponent.SetValueAsBool` _returnvalue "CanSeePlayer" _bsuccessfullysensed)
      (if (not _bsuccessfullysensed)
        (`BlackboardComponent.SetValueAsVector` _returnvalue "LastSeenLocation" _returnvalue_2)
        (`KismetSystemLibrary.DrawDebugSphere` _returnvalue_2 100.0 12 (struct :`R` 1.0 :`G` 1.0 :`B` 1.0 :`A` 1.0) 5.0 1.0)))))

(fn `UserConstructionScript`)